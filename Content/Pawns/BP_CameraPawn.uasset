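; BP_CameraPawn is a camera pawn that pans across the world when the cursor nears the screen edges.
; The MouseX and MouseY axis events compare the cursor position, as a fraction of viewport size, against EdgeMin and EdgeMax thresholds.
; Past a threshold, the pawn moves along world Y for horizontal edges or world X for vertical edges, at ScrollSpeed scaled by delta time.
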(event `InputAxisKey|MouseX`
  (params (AxisValue :type "Float (single-precision)"))
  (bind (_returnvalue_x _returnvalue_y) (`KismetMathLibrary.BreakVector2D` (`WidgetLayoutLibrary.GetViewportSize`)))
  (bind _returnvalue (* (`self.ScrollSpeed`) (`GameplayStatics.GetWorldDeltaSeconds`)))
  (bind _returnvalue_2 (/ (`PlayerController.GetMousePosition` (`GameplayStatics.GetPlayerController` 0)) _returnvalue_x))
  ; Edge Scrolling
  (if (> _returnvalue_2 (`self.EdgeMax`))
    (`self.K2_AddActorWorldOffset` (`KismetMathLibrary.MakeVector` 0.0 _returnvalue))
    (elif (< _returnvalue_2 (`self.EdgeMin`))
      (`self.K2_AddActorWorldOffset` (`KismetMathLibrary.MakeVector` 0.0 (* _returnvalue -1.0))))))

(event `InputAxisKey|MouseY`
  (params (AxisValue :type "Float (single-precision)"))
  (bind (_returnvalue_x _returnvalue_y) (`KismetMathLibrary.BreakVector2D` (`WidgetLayoutLibrary.GetViewportSize`)))
  (bind _returnvalue (* (`self.ScrollSpeed`) (`GameplayStatics.GetWorldDeltaSeconds`)))
  (bind _returnvalue_2 (/ (`.LocationY` (`PlayerController.GetMousePosition` (`GameplayStatics.GetPlayerController` 0))) _returnvalue_y))
  ; Edge Scrolling
  (if (> _returnvalue_2 (`self.EdgeMax`))
    (`self.K2_AddActorWorldOffset` (`KismetMathLibrary.MakeVector` (* _returnvalue -1.0)))
    (elif (< _returnvalue_2 (`self.EdgeMin`))
      (`self.K2_AddActorWorldOffset` (`KismetMathLibrary.MakeVector` _returnvalue)))))

(fn `UserConstructionScript`)