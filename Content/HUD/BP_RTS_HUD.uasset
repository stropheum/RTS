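; RTS HUD that handles drag-box (marquee) unit selection and shows selection debug text.
; Marquee press, hold and release events track mouse positions and call selection handlers defined outside this graph.
; DrawHUD renders the translucent box and, while selecting, updates the group of BP_SelectableUnitBase units and marks pending ones.
; A debug widget created at BeginPlay receives passive and active selection strings every Tick.
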(event `SelectableUnitInterface.MarqueePressed`
  (bind (_locationx _locationy) (`PlayerController.GetMousePosition` (`GameplayStatics.GetPlayerController` 0)))
  ; Marquee Selection Start
  (`self.HandleMarqueeSelectionPressed`)
  (set `self.MouseStartPosition` (`KismetMathLibrary.MakeVector2D` _locationx _locationy)))

(event `SelectableUnitInterface.MarqueeHeld`
  (bind (_locationx _locationy) (`PlayerController.GetMousePosition` (`GameplayStatics.GetPlayerController` 0)))
  ; Marquee Selection Held
  (set `self.MouseCurrentPosition` (`KismetMathLibrary.MakeVector2D` _locationx _locationy)))

(event `SelectableUnitInterface.MarqueeReleased`
  (`self.HandleMarqueeSelectionReleased`))

(event `self.ReceiveDrawHUD`
  (params (SizeX :type Integer) (SizeY :type Integer))
  ; Draw Marquee While Actively Selecting
  ;; Render Selection Reticle
  (`self.RenderSelectionBox` (struct :`G` 1.0 :`B` 0.52549 :`A` 0.2))
  (if (`self.IsSelecting`)
    (`self.UpdateSelectionGroup` "/Game/Characters/BP_SelectableUnitBase.BP_SelectableUnitBase_C")
    ;; Update Selected group and select them
    (for _array_element (`self.PendingSelectedActors`)
      (message `SelectableUnitInterface.SetSelectionState` _array_element "Pending"))))

(event `self.ReceiveTick`
  (params (DeltaSeconds :type "Float (single-precision)"))
  (bind _returnvalue (`self.PassiveSelectionToString`))
  (`/Game/Widgets/DB_DebugWidget.SetPassiveText` (stale `self.ReceiveBeginPlay` _returnvalue) (`KismetTextLibrary.Conv_StringToText` _returnvalue))
  (bind _returnvalue_2 (`self.ActiveSelectionToString`))
  (`/Game/Widgets/DB_DebugWidget.SetActiveText` (stale `self.ReceiveBeginPlay` _returnvalue) (`KismetTextLibrary.Conv_StringToText` _returnvalue_2)))

(event `self.ReceiveBeginPlay`
  (bind _returnvalue (`|CreateWidget` "/Game/Widgets/DB_DebugWidget.DB_DebugWidget_C" (`self.PlayerOwner`)))
  (`UserWidget.AddToViewport` _returnvalue 0))

(fn `UserConstructionScript`)