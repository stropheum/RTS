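; BP_CommandReticle is a short-lived decal actor that, going by its name, marks a command with an animated reticle.
; It caches the decal's world scale on BeginPlay, then accumulates elapsed time on Tick to drive two back-to-back linear scale lerps, each with its own duration and target scale.
; The actor destroys itself once both phases have finished.
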(event `self.ReceiveBeginPlay`
  (set `self.StartingScale` (`SceneComponent.K2_GetComponentScale` (`self.Decal`))))

(event `self.ReceiveTick`
  (params (DeltaSeconds :type "Float (single-precision)"))
  (if (`KismetSystemLibrary.IsValid` (`self.Decal`))
    (set `self.ElapsedTime` (+ DeltaSeconds (`self.ElapsedTime`)))
    ; Phase 1 Lerp
    (if (< (`self.ElapsedTime`) (`self.Phase 1 Duration`))
      (`SceneComponent.SetWorldScale3D` (`self.Decal`) (`KismetMathLibrary.VLerp` (`self.StartingScale`) (`self.Phase 1 Scale`) (/ (`self.ElapsedTime`) (`self.Phase 1 Duration`))))
      (else
        ; Phase 2 Lerp
        (if (< (`self.ElapsedTime`) (+ (`self.Phase 1 Duration`) (`self.Phase 2 Duration`)))
          (`SceneComponent.SetWorldScale3D` (`self.Decal`) (`KismetMathLibrary.VLerp` (`self.Phase 1 Scale`) (`self.Phase 2 Scale`) (/ (- (`self.ElapsedTime`) (`self.Phase 1 Duration`)) (`self.Phase 2 Duration`))))
          (else
            (`self.K2_DestroyActor`)))))))

(fn `UserConstructionScript`)