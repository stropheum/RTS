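; BP_SelectableUnitBase is a base Blueprint for units that can be selected and commanded to move.
; BeginPlay creates a dynamic material for SelectionDecal, which SetSelectionState uses to hide the decal when unselected or show it white for pending and teal-green for selected.
; Command handles Move by stopping the AI controller's current movement and issuing AIMoveTo to the given location.
; SelectUnit and DeselectUnit are empty events.
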(event `self.ReceiveBeginPlay`
  (bind _returnvalue (`DecalComponent.CreateDynamicMaterialInstance` (`self.SelectionDecal`)))
  (set `self.DecalMaterialInstance` _returnvalue))

(event `SelectableUnitInterface.SelectUnit`)

(event `SelectableUnitInterface.DeselectUnit`)

(event `SelectableUnitInterface.SetSelectionState`
  (params (State :type "ESelectionState Enum" :default "NotSelected"))
  (bind _decalmaterialinstance (`self.DecalMaterialInstance`))
  (switch `ESelectionState` State
    (:`NotSelected`
      (`SceneComponent.SetVisibility` (`self.SelectionDecal`) false false)
      (`MaterialInstanceDynamic.SetVectorParameterValue` _decalmaterialinstance "DecalColor" (struct :`R` 1.0 :`G` 1.0 :`B` 1.0 :`A` 0.6) :!label _label))
    (:`Pending`
      (`SceneComponent.SetVisibility` (`self.SelectionDecal`) true false)
      (goto _label))
    (:`Selected`
      (`SceneComponent.SetVisibility` (`self.SelectionDecal`) true false)
      (`MaterialInstanceDynamic.SetVectorParameterValue` _decalmaterialinstance "DecalColor" (struct :`G` 1.0 :`B` 0.695535 :`A` 0.6)))))

(event `CommandableInterface.Command`
  (params (Command :type "ECommand Enum" :default "None") (Location :type "Vector Structure (by ref)"))
  (bind _returnvalue (`AIBlueprintHelperLibrary.GetAIController` self))
  (switch `ECommand` Command
    (:`Move`
      (`Controller.StopMovement` _returnvalue)
      (`AITask_MoveTo.AIMoveTo` _returnvalue Location null))))

(fn `UserConstructionScript`)