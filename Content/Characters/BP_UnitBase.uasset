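; Base character for a commandable unit with selection feedback and AI-driven movement.
; Selection state sets the visibility and color of a ground decal through a dynamic material instance, separating not selected, pending and selected.
; A Move command stops current movement, runs AIMoveTo to the location and toggles ShouldMove on the cached ABP_Manny anim instance.
; Tick copies the AI controller's nav movement velocity into that anim instance.
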(event `self.ReceiveBeginPlay`
  (bind _asabp_manny (cast `/Game/Characters/Mannequins/Animations/ABP_Manny` (`SkeletalMeshComponent.GetAnimInstance` (`self.Mesh`))))
  (set `self.CachedAnimInstance` _asabp_manny)
  (bind _returnvalue (`DecalComponent.CreateDynamicMaterialInstance` (`self.Decal`)))
  (set `self.DecalMaterialInstance` _returnvalue))

(event `SelectableUnitInterface.SelectUnit`)

(event `SelectableUnitInterface.DeselectUnit`)

(event `SelectableUnitInterface.SetSelectionState`
  (params (State :type "ESelectionState Enum" :default "NotSelected"))
  (bind _decal (`self.Decal`))
  (bind _decalmaterialinstance (`self.DecalMaterialInstance`))
  (switch `ESelectionState` State
    (:`NotSelected`
      (`SceneComponent.SetVisibility` _decal false false)
      (`MaterialInstanceDynamic.SetVectorParameterValue` _decalmaterialinstance "DecalColor" (struct :`R` 1.0 :`G` 1.0 :`B` 1.0 :`A` 0.6) :!label _label))
    (:`Pending`
      (`SceneComponent.SetVisibility` _decal true false)
      (goto _label))
    (:`Selected`
      (`SceneComponent.SetVisibility` _decal true false)
      (`MaterialInstanceDynamic.SetVectorParameterValue` _decalmaterialinstance "DecalColor" (struct :`G` 1.0 :`B` 0.695535 :`A` 0.6)))))

(event `CommandableInterface.Command`
  (params (Command :type "ECommand Enum" :default "None") (Location :type "Vector Structure (by ref)"))
  (bind _cachedaniminstance (`self.CachedAnimInstance`))
  (bind _returnvalue (`AIBlueprintHelperLibrary.GetAIController` self))
  (switch `ECommand` Command
    (:`Move`
      (`Controller.StopMovement` _returnvalue)
      (`AITask_MoveTo.AIMoveTo` _returnvalue Location null -1.0 "Default" "Default" true false
        (:`then`
          (set `/Game/Characters/Mannequins/Animations/ABP_Manny.ShouldMove` true _cachedaniminstance))
        (:`OnMoveFinished`
          (set `/Game/Characters/Mannequins/Animations/ABP_Manny.ShouldMove` false _cachedaniminstance))))))

(event `self.ReceiveTick`
  (params (DeltaSeconds :type "Float (single-precision)"))
  (bind _returnvalue (message `NavMovementInterface.GetVelocityForNavMovement` (`AIBlueprintHelperLibrary.GetAIController` self)))
  (set `/Game/Characters/Mannequins/Animations/ABP_Manny.Velocity` _returnvalue (`self.CachedAnimInstance`)))

(fn `UserConstructionScript`)